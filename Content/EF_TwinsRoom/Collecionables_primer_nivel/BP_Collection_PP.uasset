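; BP_Collection_PP is a spinning collectible that increases the player's CollectionCounterPP by one when touched.
; Tick rotates the root component, and overlap casts to MyCharacter_New before updating the counter and showing Widget_Collector_PP.
; DestroyActor runs first on pickup, so the later Delay that should remove the widget and destroy again follows the actor's destruction and likely never completes.
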(event EventBeginPlay)

(event Collision|EventActorBeginOverlap
  (params (OtherActor :type Actor%20Object%20Reference))
  (bind _asmy_character_new (Utilities|Casting|CastToMyCharacter_New OtherActor))
  (Actor|DestroyActor self)
  (Variables|/Game/Blueprints/MyCharacter_New.MyCharacter_New_C|SetCollectionCounter_PP _asmy_character_new (+ (Variables|/Game/Blueprints/MyCharacter_New.MyCharacter_New_C|GetCollectionCounter_PP _asmy_character_new) 1))
  (bind _returnvalue (UserInterface|CreateWidget "/Game/EF_TwinsRoom/Collecionables_primer_nivel/Widget_Collector_PP.Widget_Collector_PP_C"))
  (UserInterface|Viewport|AddtoPlayerScreen _returnvalue)
  (Utilities|FlowControl|Delay 0.5)
  (Widget|RemovefromParent _returnvalue)
  (Actor|DestroyActor self))

(event EventTick
  (params (DeltaSeconds :type Float%20%28single-precision%29))
  (Transformation|AddLocalRotation (Variables|Default|GetDefaultSceneRoot) "0,1.000000, 0" false false))

(fn ConstructionScript)